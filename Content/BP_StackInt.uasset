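; BP_StackInt is a keyboard-driven test Blueprint for an integer stack whose operations are defined outside this graph.
; On BeginPlay it enables input from the first player controller.
; Q pushes the current size as a new element via Emplace, while W, E, R and T call Pop, Empty, Size and Top.
; The results of the R and T queries are not used in the graph.
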(event EventBeginPlay
  (Input|EnableInput (Game|GetPlayerController 0)))

(event Input|KeyboardEvents|T
  (params (Key :type Key%20Structure :default "None"))
  (:Pressed
    (Class|CPPStackInt|Top)))

(event Input|KeyboardEvents|Q
  (params (Key :type Key%20Structure :default "None"))
  (:Pressed
    (bind _returnvalue (Class|CPPStackInt|Size))
    (Class|CPPStackInt|Emplace _returnvalue)))

(event Input|KeyboardEvents|W
  (params (Key :type Key%20Structure :default "None"))
  (:Pressed
    (Class|CPPStackInt|Pop)))

(event Input|KeyboardEvents|E
  (params (Key :type Key%20Structure :default "None"))
  (:Pressed
    (Class|CPPStackInt|Empty)))

(event Input|KeyboardEvents|R
  (params (Key :type Key%20Structure :default "None"))
  (:Pressed
    (Class|CPPStackInt|Size)))

(fn ConstructionScript)