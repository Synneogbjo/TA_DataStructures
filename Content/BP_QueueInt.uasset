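; BP_QueueInt is a keyboard-driven harness that exercises integer queue operations.
; On BeginPlay it enables input from player controller 0, so hotkeys can call the queue functions, which are defined outside this graph.
; Z emplaces a copy of the back element's value, or zero when Back returns nothing valid.
; Other keys call Dequeue, Empty, Size, Front and Back without using any results.
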(event EventBeginPlay
  (Input|EnableInput (Game|GetPlayerController 0)))

(event Input|KeyboardEvents|N
  (params (Key :type Key%20Structure :default "None"))
  (:Pressed
    (Class|CPPQueueInt|Back)))

(event Input|KeyboardEvents|Z
  (params (Key :type Key%20Structure :default "None"))
  (:Pressed
    (bind _returnvalue (Class|CPPQueueInt|Back))
    (Utilities|IsValid _returnvalue
      (:Is%20Valid
        (Class|CPPQueueInt|Emplace (Variables|/Script/TA_DataStructures.CPP_QueueIntNode|Getvalue _returnvalue)))
      (:Is%20Not%20Valid
        (Class|CPPQueueInt|Emplace)))))

(event Input|KeyboardEvents|X
  (params (Key :type Key%20Structure :default "None"))
  (:Pressed
    (Class|CPPQueueInt|Dequeue)))

(event Input|KeyboardEvents|C
  (params (Key :type Key%20Structure :default "None"))
  (:Pressed
    (Class|CPPQueueInt|Empty)))

(event Input|KeyboardEvents|V
  (params (Key :type Key%20Structure :default "None"))
  (:Pressed
    (Class|CPPQueueInt|Size)))

(event Input|KeyboardEvents|B
  (params (Key :type Key%20Structure :default "None"))
  (:Pressed
    (Class|CPPQueueInt|Front)))

(fn ConstructionScript)